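; In-world settings menu for the CV22 hoist sim, with levers for day/night, dust and kick.
; BeginPlay caches the directional light's intensity and sets the levers' starting values.
; Dust and kick levers write scaled factors to the GameMode; day/night toggles its IsNight flag, directional lighting, sky sphere and skylight.
; LeftActor and EnteredActor hide and show the Scene component, without propagating to children.
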(event OnLeverWasChanged(LeverKick)
  (params (value :type Integer))
  (bind _ascv22hoist_sim_game_mode_base (Utilities|Casting|CastToCV22HoistSimGameModeBase (Game|GetGameMode)))
  (Variables|/Script/CV22HoistSim.CV22HoistSimGameModeBase|SetKickFactor _ascv22hoist_sim_game_mode_base (/ (Math|Conversions|ToFloat(Integer) value) 1e+02)))

(event OnLeverWasChanged(LeverDust)
  (params (value :type Integer))
  (bind _ascv22hoist_sim_game_mode_base (Utilities|Casting|CastToCV22HoistSimGameModeBase (Game|GetGameMode)))
  (Variables|/Script/CV22HoistSim.CV22HoistSimGameModeBase|SetDustFactor _ascv22hoist_sim_game_mode_base (/ (Math|Conversions|ToFloat(Integer) value) 1e+02)))

(event OnLeverWasChanged(LeverDayNight)
  (params (value :type Integer))
  (bind _returnvalue (Actor|GetActorOfClass "/Script/Engine.DirectionalLight"))
  (if (Math|Conversions|ToBoolean(Integer) value)
    (Rendering|Components|Light|SetIntensity (Variables|/Script/Engine.Light|GetLightComponent _returnvalue) 0.0)
    (Class|LightComponent|SetIndirectLightingIntensity (Variables|/Script/Engine.Light|GetLightComponent _returnvalue) 0.0)
    (bind _returnvalue_2 (Actor|GetActorOfClass "/Engine/EngineSky/BP_Sky_Sphere.BP_Sky_Sphere_C"))
    (Rendering|SetActorHiddenInGame _returnvalue_2 true)
    (bind _returnvalue_3 (Actor|GetActorOfClass "/Script/Engine.SkyLight"))
    (Rendering|SetActorHiddenInGame _returnvalue_3 true)
    (bind _ascv22hoist_sim_game_mode_base (Utilities|Casting|CastToCV22HoistSimGameModeBase (Game|GetGameMode))
      (:then
        (Variables|/Script/CV22HoistSim.CV22HoistSimGameModeBase|SetIsNight _ascv22hoist_sim_game_mode_base true))
      (:CastFailed
        (Development|PrintString "Error Castng GameMode")))
    (else
      (Rendering|Components|Light|SetIntensity (Variables|/Script/Engine.Light|GetLightComponent _returnvalue) (Variables|Default|GetDayIntensity))
      (Class|LightComponent|SetIndirectLightingIntensity (Variables|/Script/Engine.Light|GetLightComponent _returnvalue) 1.0)
      (bind _returnvalue_4 (Actor|GetActorOfClass "/Engine/EngineSky/BP_Sky_Sphere.BP_Sky_Sphere_C"))
      (Rendering|SetActorHiddenInGame _returnvalue_4 false)
      (bind _returnvalue_5 (Actor|GetActorOfClass "/Script/Engine.SkyLight"))
      (Rendering|SetActorHiddenInGame _returnvalue_5 false)
      (bind _ascv22hoist_sim_game_mode_base_2 (Utilities|Casting|CastToCV22HoistSimGameModeBase (Game|GetGameMode))
        (:then
          (Variables|/Script/CV22HoistSim.CV22HoistSimGameModeBase|SetIsNight _ascv22hoist_sim_game_mode_base_2 false))
        (:CastFailed
          (Development|PrintString "Error Castng GameMode"))))))

(event EventBeginPlay
  (bind _returnvalue (Actor|GetActorOfClass "/Script/Engine.DirectionalLight"))
  (Variables|Default|SetDayIntensity (Variables|/Script/Engine.LightComponentBase|GetIntensity (Variables|/Script/Engine.Light|GetLightComponent _returnvalue)))
  (Class|Lever|SetLeverValue (Variables|Default|GetLeverDayNight))
  (Class|Lever|SetLeverValue (Variables|Default|GetLeverDust) 50)
  (Class|Lever|SetLeverValue (Variables|Default|GetLeverKick) 50))

(event Collision|EventActorBeginOverlap
  (params (OtherActor :type Actor%20Object%20Reference)))

(event EventTick
  (params (DeltaSeconds :type Float%20%28single-precision%29)))

(event EventLeftActor
  (params (pawn :type Pawn%20Object%20Reference))
  (Rendering|SetVisibility (Variables|Default|GetScene) false false))

(event EventEnteredActor
  (params (pawn :type Pawn%20Object%20Reference))
  (Rendering|SetVisibility (Variables|Default|GetScene) true false))

(fn ConstructionScript)

(fn GetComponenttoAttachto
  (return 0))